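; Puzzle player Blueprint for a 3D Picross game that starts on BeginPlay and adds Niagara effects for puzzle progress.
; When a row is revealed, it attaches a burst to the grid root, centered along that row's axis.
; Per-axis selects derive the effect's offset and size from puzzle dimensions and block size, also passing the axis vector.
; Solving the puzzle spawns a separate effect sized to the whole grid.
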(event EventBeginPlay
  (Class|PuzzlePlayer|Start))

(event EventOnPuzzleSolvedBP
  (bind _returnvalue (Class|PuzzlePlayer|GetPuzzleGrid))
  (bind _returnvalue_2 (Niagara|SpawnSystemAttached "/Game/Picross/Common/VFX/NS_PuzzleSolved.NS_PuzzleSolved" (Variables|/Script/Picross.PuzzleGrid|GetRoot _returnvalue) "None" "0, 0, 0" "0, 0, 0" "KeepRelativeOffset" false))
  (Effects|Components|ParticleSystem|SetVectorParameter _returnvalue_2 "PuzzleSize" (* (Math|Conversions|ToVector(Float) (Utilities|Struct|BreakPuzzleDef (Variables|Default|GetPuzzleDef))) (Variables|/Script/Picross.PuzzleBlockMeshSet|GetBlockSize (Variables|/Script/Picross.PuzzleGrid|GetBlockMeshSet _returnvalue)))))

(event EventOnRowRevealedBP
  (params (Row :type Puzzle%20Row%20Structure))
  (bind _axis (Utilities|Struct|BreakPuzzleRow Row))
  (bind (_position _axis_2) (Utilities|Struct|BreakPuzzleRow Row))
  (bind _returnvalue (Class|PuzzlePlayer|GetPuzzleGrid))
  (bind _returnvalue_2 (Class|PuzzlePlayer|GetPuzzleGrid))
  (bind _puzzledef (Variables|Default|GetPuzzleDef))
  (bind _puzzledef_2 (Variables|Default|GetPuzzleDef))
  (bind _dimensions (Utilities|Struct|BreakPuzzleDef _puzzledef_2))
  (bind _dimensions_2 (Utilities|Struct|BreakPuzzleDef _puzzledef))
  (bind _returnvalue_3 (Math|Conversions|ToVector(Float) _position))
  (bind _returnvalue_4 (== _axis 2))
  (bind _returnvalue_5 (== _axis 0))
  (bind _returnvalue_6 (== _axis 1))
  (bind _blockmeshset (Variables|/Script/Picross.PuzzleGrid|GetBlockMeshSet _returnvalue))
  (bind _blockmeshset_2 (Variables|/Script/Picross.PuzzleGrid|GetBlockMeshSet _returnvalue_2))
  (bind _returnvalue_7 (Math|Conversions|ToVector(Float) _dimensions))
  (bind _returnvalue_8 (Math|Conversions|ToVector(Float) _dimensions_2))
  (bind _returnvalue_9 (+ _returnvalue_3 "0.500000,0.500000,0.500000"))
  (bind _blocksize (Variables|/Script/Picross.PuzzleBlockMeshSet|GetBlockSize _blockmeshset))
  (bind _blocksize_2 (Variables|/Script/Picross.PuzzleBlockMeshSet|GetBlockSize _blockmeshset_2))
  (bind (_x _y _z) (Math|Vector|BreakVector _blocksize_2))
  (bind _returnvalue_10 (* _returnvalue_8 0.5))
  (bind _returnvalue_11 (* _returnvalue_7 _blocksize_2))
  (bind _returnvalue_12 (- _returnvalue_9 _returnvalue_10))
  (bind _returnvalue_13 (* _returnvalue_12 _blocksize))
  (bind _returnvalue_14 (Niagara|SpawnSystemAttached "/Game/Picross/Common/VFX/NS_PuzzleRowSolved.NS_PuzzleRowSolved" (Variables|/Script/Picross.PuzzleGrid|GetRoot (Class|PuzzlePlayer|GetPuzzleGrid)) "None" (Math|Vector|MakeVector (Math|Float|SelectFloat 0.0 (.x _returnvalue_13) (== _axis_2 0)) (Math|Float|SelectFloat 0.0 (.y _returnvalue_13) (== _axis_2 1)) (Math|Float|SelectFloat 0.0 (.z _returnvalue_13) (== _axis_2 2))) "0, 0, 0" "KeepRelativeOffset" false))
  (Effects|Components|ParticleSystem|SetVectorParameter _returnvalue_14 "PuzzleSize" (Math|Vector|MakeVector (Math|Float|SelectFloat (.x _returnvalue_11) _x _returnvalue_5) (Math|Float|SelectFloat (.y _returnvalue_11) _y _returnvalue_6) (Math|Float|SelectFloat (.z _returnvalue_11) _z _returnvalue_4)))
  (Effects|Components|ParticleSystem|SetVectorParameter _returnvalue_14 "RowAxisVector" (Math|Vector|MakeVector (Math|Conversions|ToFloat(Boolean) _returnvalue_5) (Math|Conversions|ToFloat(Boolean) _returnvalue_6) (Math|Conversions|ToFloat(Boolean) _returnvalue_4))))

(fn ConstructionScript)